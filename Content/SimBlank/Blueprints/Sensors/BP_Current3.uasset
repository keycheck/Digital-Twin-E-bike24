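; BP_Current3 is a current sensor display that holds logic to show a ThingSpeak reading on a TextRender, though that logic is disconnected.
; BeginPlay only creates NewWidgetBlueprint and adds it to the viewport.
; The unwired HTTP GET chain parses the channel's JSON feeds and writes each field2 value with an "A" suffix, leaving the last visible, or shows a connection error on failure.
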(event EventBeginPlay
  (bind _returnvalue (UserInterface|CreateWidget "/Game/UI_HUD/NewWidgetBlueprint.NewWidgetBlueprint_C"))
  (UserInterface|Viewport|AddtoViewport _returnvalue 0))

(fn ConstructionScript)