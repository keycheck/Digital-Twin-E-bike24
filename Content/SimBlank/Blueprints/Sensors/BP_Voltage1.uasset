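; BP_Voltage1 is a sensor display that shows a voltage reading fetched from a ThingSpeak channel.
; On BeginPlay it sends a single HTTP GET for field 1 and parses the returned JSON feeds array.
; Each entry's value is written to a TextRender with a "V" suffix, so the last entry remains visible.
; A failed request shows a not-connected error on the same text.
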(event EventBeginPlay
  (bind _result_body (|HttpRequest "https://api.thingspeak.com/channels/2531296/fields/1.json?api_key=XC92OQ33DCA3VSMU" "Get")
    (:On%20Success
      (bind _outjsonobject (Class|JsonBlueprintFunctionLibrary|FromString _result_body))
      (bind _outvalue (|GetJsonField _outjsonobject "feeds"))
      (for _array_element _outvalue
        (bind _outvalue_2 (|GetJsonField _array_element "field1"))
        (Development|PrintString "reached get")
        (Rendering|Components|TextRender|SetText (Variables|Default|GetTextRender) (Utilities|Text|ToText(String) (Utilities|String|Append _outvalue_2 "V")))))
    (:On%20Error
      (bind _output_get (Variables|Default|SeterrorText "ERROR- Not Connected"))
      (Rendering|Components|TextRender|SetText (Variables|Default|GetTextRender) (Utilities|Text|ToText(String) _output_get)))))

(fn ConstructionScript)